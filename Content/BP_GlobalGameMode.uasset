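; BP_GlobalGameMode is the game mode that passes the expected player count into the game state for the CaiNaoCaiLevel map.
; On BeginPlay it compares the current level name and, on that map only, copies ExpectedPlayers from BP_GlobalGameInstance into RequiredPlayers on BP_GlobalGameState.
; It prints the resulting count as debug output and does nothing on other levels.
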(event EventBeginPlay
  (bind _returnvalue (Game|GetCurrentLevelName true))
  (if (Utilities|Enum|Equal(Enum) _returnvalue "CaiNaoCaiLevel")
    (bind _asbp_global_game_instance (Utilities|Casting|CastToBP_GlobalGameInstance (Game|GetGameInstance)))
    (bind _asbp_global_game_state (Utilities|Casting|CastToBP_GlobalGameState (Game|GetGameState)))
    (bind _output_get (Variables|/Game/BP_GlobalGameState.BP_GlobalGameState_C|SetRequired%20Players _asbp_global_game_state (Variables|/Game/BP_GlobalGameInstance.BP_GlobalGameInstance_C|GetExpected%20Players _asbp_global_game_instance)))
    (Development|PrintString (Utilities|String|Append "required:" (Utilities|String|ToString(Integer) _output_get)))))

(fn ConstructionScript)