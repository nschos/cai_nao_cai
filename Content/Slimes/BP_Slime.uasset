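; Slime actor that squashes and jiggles on hard impacts and can be snapped onto a treadmill.
; Sphere hits above an impulse threshold play a squash timeline, then a decaying-or-curved sine jiggle timeline, with a flag blocking retriggers until shortly afterward.
; Both timelines feed UpdateSlimeVisual, which scales the mesh, offsetting Z opposite to XY.
; SnapToTreadmill disables physics, eases the mesh to a target location and attaches the actor to the treadmill.
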(event OnComponentHit(Sphere)
  (params (HitComponent :type Primitive%20Component%20Object%20Reference) (OtherActor :type Actor%20Object%20Reference) (OtherComp :type Primitive%20Component%20Object%20Reference) (NormalImpulse :type Vector :default "0, 0, 0") (Hit :type Hit%20Result%20Structure%20%28by%20ref%29))
  (if (and (> (Math|Vector|VectorLength NormalImpulse) (Variables|Default|GetImpactThresold)) (not (Variables|Default|GetIsSquashing)))
    (Variables|Default|SetIsSquashing true)
    (bind _squasalpha (Timeline|TL_SlimeSquash PlayFromStart)
      (:Update
        (Variables|Default|SetSquashScale (Math|Vector|Lerp(Vector) (Variables|Default|GetOriginalScale) (* (Variables|Default|GetOriginalScale) "1.100000,1.100000,0.900000") _squasalpha))
        (CallFunction|UpdateSlimeVisual :!label _label))
      (:Finished
        (bind _jiggleintensity (Timeline|TL_SlimeJiggle PlayFromStart)
          (:Update
            (bind _output_get (Variables|Default|SetJiggleOffset (* (* (Math|Trig|Sin(Radians) (* (Components|Timeline|GetPlaybackPosition (Variables|Default|GetTL_SlimeJiggle)) 18.0)) (Variables|Default|GetJiggleAmplitude)) _jiggleintensity)))
            (goto _label))
          (:Finished
            (Utilities|FlowControl|Delay 0.2)
            (Variables|Default|SetIsSquashing false)))))))

(event Custom|SnapToTreadmill
  (params (TargetLocation :type Vector) (Target%20Treadmill :type Actor%20Object%20Reference))
  (bind _slimemesh (Variables|Default|GetSlimeMesh))
  (Physics|SetSimulatePhysics _slimemesh false)
  (Components|MoveComponentTo _slimemesh TargetLocation "0, 0, 0" true false 0.2 false)
  (Transformation|AttachActorToActor Target%20Treadmill "None" "KeepWorld" "KeepWorld" "KeepWorld" true))

(event EventBeginPlay
  (Variables|Default|SetOriginalScale (Variables|/Script/Engine.SceneComponent|GetRelativeScale3D (Variables|Default|GetSlimeMesh)))
  (Variables|Default|SetSquashScale (Variables|Default|GetOriginalScale)))

(event Collision|EventActorBeginOverlap
  (params (OtherActor :type Actor%20Object%20Reference)))

(event EventTick
  (params (DeltaSeconds :type Float%20%28single-precision%29)))

(fn ConstructionScript)

(fn UpdateSlimeVisual
  (bind _jiggleoffset (Variables|Default|GetJiggleOffset))
  (bind _returnvalue (+ 1.0 _jiggleoffset))
  (Transformation|SetRelativeScale3D (Variables|Default|GetSlimeMesh) (* (Math|Vector|MakeVector _returnvalue _returnvalue (- 1.0 _jiggleoffset)) (Variables|Default|GetSquashScale))))