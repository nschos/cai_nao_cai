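; BP_Slime1 is a slime actor that squashes, stretches and pulses as it falls and hits things.
; Hard sphere hits spike a decaying JiggleOffset that drives the dynamic material's pulse intensity, with mostly upward impulses also triggering a brief squash.
; Tick eases mesh scale toward that squash, or toward a vertical stretch based on downward velocity.
; UpdateSlimeVisual offers jiggle-based scaling but is not called within this Blueprint.
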(event OnComponentHit(Sphere)
  (params (HitComponent :type Primitive%20Component%20Object%20Reference) (OtherActor :type Actor%20Object%20Reference) (OtherComp :type Primitive%20Component%20Object%20Reference) (NormalImpulse :type Vector :default "0, 0, 0") (Hit :type Hit%20Result%20Structure%20%28by%20ref%29))
  (bind _returnvalue (Math|Vector|VectorLength NormalImpulse))
  (if (and (and (> _returnvalue (Variables|Default|GetImpactThresold)) (not (Variables|Default|GetIsSquashing))) (< (Variables|Default|GetJiggleOffset) 0.06))
    (Variables|Default|SetJiggleOffset 1.4)
    (if (> (.Z (Math|Vector|BreakVector NormalImpulse)) (* _returnvalue 0.4))
      (Variables|Default|SetIsSquashing true)
      (Utilities|FlowControl|Delay 0.12)
      (Variables|Default|SetIsSquashing false))))

(event EventBeginPlay
  (bind _slimemesh (Variables|Default|GetSlimeMesh))
  (Variables|Default|SetOriginalScale (Variables|/Script/Engine.SceneComponent|GetRelativeScale3D _slimemesh))
  (Variables|Default|SetJiggleOffset 0.0)
  (Variables|Default|SetIsSquashing false)
  (bind _returnvalue (Rendering|Material|CreateDynamicMaterialInstance _slimemesh 0 0 "None" :!class /Script/Engine.PrimitiveComponent))
  (Rendering|Material|SetScalarParameterValue _returnvalue "Pulse Intensity" 1.0 :!class /Script/Engine.MaterialInstanceDynamic)
  (Rendering|Material|SetScalarParameterValue _returnvalue "Band Intensity" 0.25 :!class /Script/Engine.MaterialInstanceDynamic)
  (Rendering|Material|SetScalarParameterValue _returnvalue "Interactive intensity" 0.0 :!class /Script/Engine.MaterialInstanceDynamic)
  (Rendering|Material|SetScalarParameterValue _returnvalue "Panning Speed" 0.04 :!class /Script/Engine.MaterialInstanceDynamic)
  (Rendering|Material|SetScalarParameterValue _returnvalue "Pulse Speed" 0.75 :!class /Script/Engine.MaterialInstanceDynamic))

(event EventTick
  (params (DeltaSeconds :type Float%20%28single-precision%29))
  (bind _slimemesh (Variables|Default|GetSlimeMesh))
  (bind _originalscale (Variables|Default|GetOriginalScale))
  (bind _relativescale3d (Variables|/Script/Engine.SceneComponent|GetRelativeScale3D _slimemesh))
  (Variables|Default|SetJiggleOffset (Math|Interpolation|FInterpTo (Variables|Default|GetJiggleOffset) 0.0 DeltaSeconds 11.0))
  (if (Variables|Default|GetIsSquashing)
    (Transformation|SetRelativeScale3D _slimemesh (Math|Interpolation|VInterpTo _relativescale3d (* _originalscale "(X=1.12,Y=1.12,Z=0.80)") DeltaSeconds 24.0))
    (else
      (Transformation|SetRelativeScale3D _slimemesh (Math|Interpolation|VInterpTo _relativescale3d (Math|Vector|Lerp(Vector) _originalscale (* _originalscale "(X=0.94,Y=0.94,Z=1.13)") (Math|Float|MapRangeClamped (.Z (Math|Vector|BreakVector (Transformation|GetComponentVelocity (Variables|Default|GetSphere)))) -1.4e+02 -6.5e+02 0.0 1.0)) DeltaSeconds 18.0))))
  (bind _asmaterial_instance_dynamic (Utilities|Casting|CastToMaterialInstanceDynamic (Rendering|Material|GetMaterial _slimemesh 0)))
  (Rendering|Material|SetScalarParameterValue _asmaterial_instance_dynamic "Pulse Intensity" (+ (Variables|Default|GetJiggleOffset) 1.0) :!class /Script/Engine.MaterialInstanceDynamic))

(fn ConstructionScript)

(fn UpdateSlimeVisual
  (bind _jiggleoffset (Variables|Default|GetJiggleOffset))
  (bind _returnvalue (+ 1.0 _jiggleoffset))
  (Transformation|SetRelativeScale3D (Variables|Default|GetSlimeMesh) (* (Math|Vector|MakeVector _returnvalue _returnvalue (- 1.0 _jiggleoffset)) (Variables|Default|GetSquashScale))))