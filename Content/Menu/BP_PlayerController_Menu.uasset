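; BP_PlayerController_Menu is the player controller for the main menu, setting up the menu UI and camera on BeginPlay.
; It creates WB_MainMenu, adds it to the viewport, shows the mouse cursor and switches input to UI-only focused on that widget.
; It then sets the view target to actors tagged "Default", looping over all matches so the last one found becomes the final view.
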(event EventBeginPlay
  (Utilities|FlowControl|Sequence
    (:then_0
      (bind _returnvalue (UserInterface|CreateWidget "/Game/Menu/WB_MainMenu.WB_MainMenu_C"))
      (bind _output_get (Variables|Default|SetMenuRef _returnvalue))
      (Utilities|IsValid _output_get
        (:Is%20Valid
          (UserInterface|Viewport|AddtoViewport _output_get 0)
          (Variables|Default|SetbShowMouseCursor true))))
    (:then_1
      (Utilities|IsValid (Variables|Default|GetMenuRef)
        (:Is%20Valid
          (Input|SetInputModeUIOnly (Game|GetPlayerController 0) (Variables|Default|GetMenuRef) "DoNotLock" false))))
    (:then_2
      (bind _outactors (Actor|GetAllActorswithTag "Default"))
      (for _array_element _outactors
        (Game|Player|SetViewTargetwithBlend _array_element 0.0 "VTBlend_Linear" 0.0 false)))))

(fn ConstructionScript)