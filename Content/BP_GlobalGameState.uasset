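; Game state for a turn-based multiplayer slime game that tracks which player holds the current turn.
; BeginPlay picks a random starting player, while StartTurns selects the first in PlayerArray.
; LockTurn either advances immediately or makes Tick wait until every unfallen slime stays below a speed threshold for WaitTime.
; AdvanceTurn makes the outgoing player's controller repossess its first-person character, then cycles CurrentTurnPlayer through PlayerArray.
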(event EventBeginPlay
  (bind _asbp_global_player_state (Utilities|Casting|CastToBP_GlobalPlayerState (Utilities|Array|Get(acopy) (Variables|Default|GetPlayerArray) (Math|Random|RandomInteger (Utilities|Array|Length (Variables|Default|GetPlayerArray))))))
  (Variables|Default|SetCurrentTurnPlayer _asbp_global_player_state))

(event EventTick
  (params (DeltaSeconds :type Float%20%28single-precision%29))
  (if (Variables|Default|GetIsTurnLocked)
    (bind _result (CallFunction|IsSlimesMoving))
    (if (not _result)
      (bind _output_get (Variables|Default|SetWaitCounter (+ (Variables|Default|GetWaitCounter) DeltaSeconds)))
      (if (>= _output_get (Variables|Default|GetWaitTime))
        (Development|PrintString "Advance Turn!")
        (Variables|Default|SetIsTurnLocked false)
        (CallFunction|AdvanceTurn))
      (else
        (Variables|Default|SetWaitCounter 0.0)))))

(fn ConstructionScript)

(fn OnRepRemovedSticks
  (Development|PrintString (Utilities|String|Append "Sticks removed:" (Utilities|String|ToString(Integer) (Variables|Default|GetRemovedSticks)))))

(fn StartTurns
  (Variables|Default|SetTurnIndex 0)
  (bind _asbp_global_player_state (Utilities|Casting|CastToBP_GlobalPlayerState (Utilities|Array|Get(acopy) (Variables|Default|GetPlayerArray) (Variables|Default|GetTurnIndex))))
  (Variables|Default|SetCurrentTurnPlayer _asbp_global_player_state))

(fn AdvanceTurn
  (bind _asbp_global_player_controller (Utilities|Casting|CastToBP_GlobalPlayerController (Game|GetPlayerController (Utilities|Array|Get(acopy) (Variables|Default|GetPlayerArray) (Variables|Default|GetTurnIndex)))))
  (Default|ServerPossessThirdPerson _asbp_global_player_controller (Variables|/Game/BP_GlobalPlayerController.BP_GlobalPlayerController_C|GetFirstPersonCharacter _asbp_global_player_controller) true)
  (bind _result (Math|Integer|IncrementInt (Variables|Default|GetTurnIndex))
    (:%20%20
      (Variables|Default|SetTurnIndex (Math|Integer|%(Integer) _result (Utilities|Array|Length (Variables|Default|GetPlayerArray))))
      (bind _asbp_global_player_state (Utilities|Casting|CastToBP_GlobalPlayerState (Utilities|Array|Get(acopy) (Variables|Default|GetPlayerArray) (Variables|Default|GetTurnIndex))))
      (Variables|Default|SetCurrentTurnPlayer _asbp_global_player_state))))

(fn NewFunction)

(fn LockTurn
  (if (Variables|Default|GetSkipLock)
    (CallFunction|AdvanceTurn)
    (else
      (Variables|Default|SetIsTurnLocked true)
      (Variables|Default|SetWaitCounter 0.0))))

(fn IsSlimesMoving
  (bind _outactors (Actor|GetAllActorsOfClass "/Game/Slimes/BP_Slime.BP_Slime_C"))
  (for _array_element _outactors
    (if (not (Variables|/Game/Slimes/BP_Slime.BP_Slime_C|GetFallen _array_element))
      (if (>= (+ (Math|Float|Absolute(Float) (.x (Transformation|GetVelocity _array_element))) (Math|Float|Absolute(Float) (.y (Transformation|GetVelocity _array_element))) (Math|Float|Absolute(Float) (.z (Transformation|GetVelocity _array_element)))) 5e+01)
        (return true))))
  (return false))