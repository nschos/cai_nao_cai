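; Game instance that starts and ends the multiplayer CaiNaoCai minigame and decides its winners.
; Start locks joining, shows loading screens and server-travels everyone to the game level; end notifies results, waits briefly, reopens joining and travels back to the persistent lobby.
; Scoring subtracts heavily penalized fallen balls from removed sticks per player state.
; Top scorers are flagged as winners, and a shared top score flags a tie on every player.
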(event Custom|ComputeScores
  (for _array_element (Variables|/Script/Engine.GameStateBase|GetPlayerArray (Game|GetGameState))
    (bind _asbp_global_player_state (Utilities|Casting|CastToBP_GlobalPlayerState _array_element))
    (Utilities|Array|Add (Variables|Default|GetPlayerScores) (Utilities|Struct|MakeS_PlayerScore _asbp_global_player_state (Variables|/Game/BP_GlobalPlayerState.BP_GlobalPlayerState_C|GetRemovedSticks _asbp_global_player_state) (Variables|/Game/BP_GlobalPlayerState.BP_GlobalPlayerState_C|GetFallenBalls _asbp_global_player_state) (- (Variables|/Game/BP_GlobalPlayerState.BP_GlobalPlayerState_C|GetRemovedSticks _asbp_global_player_state) (* (Variables|/Game/BP_GlobalPlayerState.BP_GlobalPlayerState_C|GetFallenBalls _asbp_global_player_state) 1000))))))

(event Custom|EndCaiNaoCaiGame
  (CallFunction|AssignPodium)
  (for _array_element (Variables|/Script/Engine.GameStateBase|GetPlayerArray (Game|GetGameState))
    (bind _asbp_global_player_state (Utilities|Casting|CastToBP_GlobalPlayerState _array_element))
    (bind _asbp_global_player_controller (Utilities|Casting|CastToBP_GlobalPlayerController (Game|GetPlayerController _asbp_global_player_state)))
    (Default|NotifyEndGame _asbp_global_player_controller (Variables|/Game/BP_GlobalPlayerState.BP_GlobalPlayerState_C|GetHasTied _asbp_global_player_state) (Variables|/Game/BP_GlobalPlayerState.BP_GlobalPlayerState_C|GetHasWon _asbp_global_player_state)))
  (Utilities|FlowControl|Delay 5.0)
  (bind _asplayer_join_game_mode (Utilities|Casting|CastToPlayerJoinGameMode (Game|GetGameMode)))
  (Class|PlayerJoinGameMode|EndCaiNaoCaiandAllowJoin _asplayer_join_game_mode)
  (for _array_element_2 (Variables|/Script/Engine.GameStateBase|GetPlayerArray (Game|GetGameState))
    (bind _asbp_global_player_state_2 (Utilities|Casting|CastToBP_GlobalPlayerState _array_element_2))
    (bind _asbp_global_player_controller_2 (Utilities|Casting|CastToBP_GlobalPlayerController (Game|GetPlayerController _asbp_global_player_state_2)))
    (Default|ShowLoadingScreen _asbp_global_player_controller_2))
  (Development|ExecuteConsoleCommand "ServerTravel LobbyMap_SessionPersistent?listen" 0))

(event Custom|AssignPodium
  (Utilities|Array|Clear (Variables|Default|GetPlayerScores))
  (Variables|Default|SetWinnerScore -99999999)
  (Variables|Default|SetTiedCount 0)
  (Variables|Default|SetTiedGame false)
  (CallFunction|ComputeScores)
  (for _array_element (Variables|Default|GetPlayerScores)
    (if (> (.Score (Utilities|Struct|BreakS_PlayerScore _array_element)) (Variables|Default|GetWinnerScore))
      (Variables|Default|SetWinnerScore (.Score (Utilities|Struct|BreakS_PlayerScore _array_element)))))
  (for _array_element_2 (Variables|Default|GetPlayerScores)
    (if (== (Variables|Default|GetWinnerScore) (.Score (Utilities|Struct|BreakS_PlayerScore _array_element_2)))
      (bind _result (Math|Integer|IncrementInt (Variables|Default|GetTiedCount))
        (:%20%20
          (Variables|Default|SetTiedCount _result)
          (Variables|/Game/BP_GlobalPlayerState.BP_GlobalPlayerState_C|SetHasWon (.PlayerState (Utilities|Struct|BreakS_PlayerScore _array_element_2)) true)))
      (else
        (Variables|/Game/BP_GlobalPlayerState.BP_GlobalPlayerState_C|SetHasWon (.PlayerState (Utilities|Struct|BreakS_PlayerScore _array_element_2)) false))))
  (if (> (Variables|Default|GetTiedCount) 1)
    (Variables|Default|SetTiedGame true)
    (else
      (Variables|Default|SetTiedGame false)))
  (for _array_element_3 (Variables|/Script/Engine.GameStateBase|GetPlayerArray (Game|GetGameState))
    (bind _asbp_global_player_state (Utilities|Casting|CastToBP_GlobalPlayerState _array_element_3))
    (Variables|/Game/BP_GlobalPlayerState.BP_GlobalPlayerState_C|SetHasTied _asbp_global_player_state (Variables|Default|GetTiedGame))))

(event Custom|StartCaiNaoCaiGame
  (bind _asplayer_join_game_mode (Utilities|Casting|CastToPlayerJoinGameMode (Game|GetGameMode)))
  (Class|PlayerJoinGameMode|StartCaiNaoCaiandLockJoin _asplayer_join_game_mode)
  (for _array_element (Variables|/Script/Engine.GameStateBase|GetPlayerArray (Game|GetGameState))
    (bind _asbp_global_player_state (Utilities|Casting|CastToBP_GlobalPlayerState _array_element))
    (bind _asbp_global_player_controller (Utilities|Casting|CastToBP_GlobalPlayerController (Game|GetPlayerController _asbp_global_player_state)))
    (if (Ability|HasAuthority _array_element)
      (Default|ShowLoadingScreen _asbp_global_player_controller)
      (else
        (Default|ShowLoadingScreen _asbp_global_player_controller))))
  (Development|ExecuteConsoleCommand "ServerTravel CaiNaoCaiLevel?listen" 0))